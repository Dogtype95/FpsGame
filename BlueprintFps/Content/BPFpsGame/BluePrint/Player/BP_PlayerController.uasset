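; BP_PlayerController is the player controller for BP_Player, turning Enhanced Input into look, movement and jump.
; It adds IMC_Player on BeginPlay and caches the possessed pawn as MyPlayer.
; Movement follows the control rotation's yaw only and is gated by the pawn's IsMove flag, exposed through getter and setter functions.
; Look input drives yaw and pitch directly, and jump calls the pawn without that gate.
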(event Input|EnhancedActionEvents|EnhancedInputActionIA_Move
  (params (ActionValue :type Vector%202D%20Structure) (ElapsedSeconds :type Float%20%28double-precision%29) (TriggeredSeconds :type Float%20%28double-precision%29) (InputAction :type Input%20Action%20Object%20Reference :default "/Game/BPFpsGame/Input/Player/IA_Move.IA_Move"))
  ;[0.15 0.15 0.15 0.5] 이동
  (if (CallFunction|GetIsMove)
    (bind _output_get (Variables|Default|SetMoveDirection ActionValue))
    (Utilities|FlowControl|Sequence
      (:then_0
        (Pawn|Input|AddMovementInput (Variables|Default|GetMyPlayer) (Math|Vector|GetRightVector (Math|Rotator|MakeRotator 0.0 0.0 (.yaw (Pawn|GetControlRotation :!class /Script/Engine.Controller)))) (.X (Math|Vector2D|BreakVector2D _output_get)) false))
      (:then_1
        (Pawn|Input|AddMovementInput (Variables|Default|GetMyPlayer) (Math|Vector|GetForwardVector (Math|Rotator|MakeRotator 0.0 0.0 (.yaw (Pawn|GetControlRotation :!class /Script/Engine.Controller)))) (.Y (Math|Vector2D|BreakVector2D _output_get)) false)))))

(event Input|EnhancedActionEvents|EnhancedInputActionIA_Look
  (params (ActionValue :type Vector%202D%20Structure) (ElapsedSeconds :type Float%20%28double-precision%29) (TriggeredSeconds :type Float%20%28double-precision%29) (InputAction :type Input%20Action%20Object%20Reference :default "/Game/BPFpsGame/Input/Player/IA_Look.IA_Look"))
  (bind (_x _y) (Math|Vector2D|BreakVector2D ActionValue))
  ;[0.15 0.15 0.15 0.5] 회전
  (Class|PlayerController|AddYawInput _x)
  (Class|PlayerController|AddPitchInput _y))

(event Input|EnhancedActionEvents|EnhancedInputActionIA_Jumping
  (params (ActionValue :type Boolean) (ElapsedSeconds :type Float%20%28double-precision%29) (TriggeredSeconds :type Float%20%28double-precision%29) (InputAction :type Input%20Action%20Object%20Reference :default "/Game/BPFpsGame/Input/Player/IA_Jumping.IA_Jumping"))
  (Character|Jump (Variables|Default|GetMyPlayer)))

(event EventBeginPlay
  (Utilities|FlowControl|Sequence
    (:then_0
      (|InputInit))))

(event EventPossess
  (params (PossessedPawn :type Pawn%20Object%20Reference))
  (Utilities|FlowControl|Sequence
    (:then_0
      (|GetMyPlayer PossessedPawn))))

(fn ConstructionScript)

(fn GetIsMove
  (bind _myplayer (Variables|Default|GetMyPlayer))
  (Utilities|IsValid _myplayer
    (:Is%20Valid
      (return (Variables|/Game/BPFpsGame/BluePrint/Player/BP_Player.BP_Player_C|GetisMove _myplayer)))))

(fn SetIsMove
  (params (isMove :type Boolean))
  (bind _myplayer (Variables|Default|GetMyPlayer))
  (Utilities|IsValid _myplayer
    (:Is%20Valid
      (Variables|/Game/BPFpsGame/BluePrint/Player/BP_Player.BP_Player_C|SetisMove _myplayer isMove))))